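; BP_UIPointTest is a test pickup actor that awards points to the player score when its box is overlapped.
; BeginPlay caches a reference to BP_TopDownGameMode.
; The first box overlap passes a DoOnce, sends a ScoreCollect message to the overlapping actor without a type check, then runs its own ScoreCollect.
; That event prints a debug string and adds ScoreToAdd through the game mode; the actor is not destroyed.
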(event `self.ReceiveBeginPlay`
  (bind _asbp_top_down_game_mode (cast `/Game/TopDown/Blueprints/BP_TopDownGameMode` (`GameplayStatics.GetGameMode`)))
  (set `self.GameModeRef` _asbp_top_down_game_mode))

(event `/Game/UI/BP_Score_Update.ScoreCollect`
  (`KismetSystemLibrary.PrintString` "points test")
  (`/Game/TopDown/Blueprints/BP_TopDownGameMode.AddPlayerScore` (`self.GameModeRef`) (`self.ScoreToAdd`)))

(event `self.Box.OnComponentBeginOverlap`
  (params (OverlappedComponent :type "PrimitiveComponent Object Reference") (OtherActor :type "Actor Object Reference") (OtherComp :type "PrimitiveComponent Object Reference") (OtherBodyIndex :type Integer) (bFromSweep :type Boolean) (SweepResult :type "HitResult Structure (by ref)"))
  (`/Engine/EditorBlueprintResources/StandardMacros.DoOnce` false
    (:`Completed`
      (message `/Game/UI/BP_Score_Update.ScoreCollect` OtherActor)
      (`/Game/UI/BP_Score_Update.ScoreCollect`))))

(fn `UserConstructionScript`)