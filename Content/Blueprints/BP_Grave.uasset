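; BP_Grave is a grave actor with active, inactive and completed states, shown by swapping the material on its Cube.
; On BeginPlay it registers itself in the GI_Graveyard game instance's InactiveGraves list.
; Activate turns it on for ActiveTime with a debug print, then reverts it and notifies the game instance through DeavtivateSpecificGrave.
; Complete flags it as completed, without cancelling that pending delayed deactivation.
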(event `self.ReceiveBeginPlay`
  (bind _output_get (set `self.GraveyardRef` (cast `/Game/Blueprints/GI_Graveyard` (`GameplayStatics.GetGameInstance`) :!pure true)))
  (`KismetArrayLibrary.Array_Add` (`/Game/Blueprints/GI_Graveyard.InactiveGraves` _output_get) self))

(event `Activate`
  (set `self.bIsActive` true)
  ;[1 1 1] TODO: Refactor after debuging
  (`PrimitiveComponent.CreateDynamicMaterialInstance` (`self.Cube`) 0 "/Game/Materials/MI_ActiveGrave.MI_ActiveGrave" "None")
  (`KismetSystemLibrary.PrintString` (`KismetStringLibrary.Concat_StrStr` (`KismetSystemLibrary.GetDisplayName` self) " is now active") true true (struct :`G` 1.0 :`B` 0.497018 :`A` 1.0) (`self.ActiveTime`))
  (`KismetSystemLibrary.Delay` (`self.ActiveTime`))
  (set `self.bIsActive` false)
  (`PrimitiveComponent.CreateDynamicMaterialInstance` (`self.Cube`) 0 "/Game/Materials/MI_InactiveGrave.MI_InactiveGrave" "None")
  (`/Game/Blueprints/GI_Graveyard.DeavtivateSpecificGrave` (`self.GraveyardRef`) self))

(event `Complete`
  (set `self.bIsCompleted` true)
  ;[1 1 1] TODO: Refactor after debuging
  (`PrimitiveComponent.CreateDynamicMaterialInstance` (`self.Cube`) 0 "/Game/Materials/MI_CompletedGrave.MI_CompletedGrave" "None"))

(fn `UserConstructionScript`)