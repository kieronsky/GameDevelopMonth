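; GI_Graveyard, apparently a Game Instance, tracks inactive graves and the count of active ones.
; ActivateRandomGrave increments the count, removes a random array entry, then calls Activate on a random pick, re-rolled after removal, so the activated grave can differ from the removed one.
; DeavtivateSpecificGrave returns a given grave to the array, decrements the count and prints a temporary debug check of the insertion.
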(event `self.ReceiveInit`)

(fn `ActivateRandomGrave`
  (bind _inactivegraves (`self.InactiveGraves`))
  (bind (_outitem _outindex) (`KismetArrayLibrary.Array_Random` _inactivegraves))
  (`/Engine/EditorBlueprintResources/StandardMacros.IncrementInt` (`self.Active Graves Amount`)
    (:`  `
      (`KismetArrayLibrary.Array_Remove` _inactivegraves _outindex)
      (`/Game/Blueprints/BP_Grave.Activate` _outitem))))

(fn `DeavtivateSpecificGrave`
  (params (GraveRef :type "/Game/Blueprints/BP_Grave Object Reference"))
  (bind _returnvalue (`KismetSystemLibrary.GetDisplayName` GraveRef))
  (bind _inactivegraves (`self.InactiveGraves`))
  (`KismetArrayLibrary.Array_Add` _inactivegraves GraveRef)
  (`/Engine/EditorBlueprintResources/StandardMacros.DecrementInt` (`self.Active Graves Amount`)
    (:`  `
      ;[1 1 1] Remove after debuging
      (if (`KismetArrayLibrary.Array_Contains` _inactivegraves GraveRef)
        (`KismetSystemLibrary.PrintString` (`KismetStringLibrary.Concat_StrStr` "Deavtivated: " _returnvalue) true true (struct :`R` 1.0 :`G` 0.015278 :`A` 1.0))
        (else
          (`KismetSystemLibrary.PrintString` (`KismetStringLibrary.Concat_StrStr` "Error! Faield at inserting  " _returnvalue) true true (struct :`R` 1.0 :`G` 0.921256 :`A` 1.0) 10.0))))))