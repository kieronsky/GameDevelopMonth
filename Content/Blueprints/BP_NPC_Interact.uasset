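; NPC interaction Blueprint that shows a text prompt while the top-down player character is nearby.
; Box overlap events cast to BP_TopDownCharacter, unhiding the Text component on entry and hiding it on exit.
; An ActivateGraveyard event, apparently a placeholder, prints a test string, calls the empty PlayerAdjustments function and shows the text.
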(event `self.Box.OnComponentBeginOverlap`
  (params (OverlappedComponent :type "PrimitiveComponent Object Reference") (OtherActor :type "Actor Object Reference") (OtherComp :type "PrimitiveComponent Object Reference") (OtherBodyIndex :type Integer) (bFromSweep :type Boolean) (SweepResult :type "HitResult Structure (by ref)"))
  ;[1 1 1] ShowInteract
  (cast `/Game/TopDown/Blueprints/BP_TopDownCharacter` OtherActor)
  (`SceneComponent.SetHiddenInGame` (`self.Text`) false false))

(event `self.Box.OnComponentEndOverlap`
  (params (OverlappedComponent :type "PrimitiveComponent Object Reference") (OtherActor :type "Actor Object Reference") (OtherComp :type "PrimitiveComponent Object Reference") (OtherBodyIndex :type Integer))
  ;[1 1 1] ShowInteract
  (cast `/Game/TopDown/Blueprints/BP_TopDownCharacter` OtherActor)
  (`SceneComponent.SetHiddenInGame` (`self.Text`) true false))

(event `/Game/Blueprints/BP_Interact.ActivateGraveyard`
  (`KismetSystemLibrary.PrintString` "Test")
  (`self.PlayerAdjustments`)
  (`SceneComponent.SetHiddenInGame` (`self.Text`) false false))

(fn `PlayerAdjustments`)

(fn `UserConstructionScript`)